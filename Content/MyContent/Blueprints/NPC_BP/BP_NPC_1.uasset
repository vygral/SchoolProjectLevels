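; BP_NPC_1 is an NPC that wanders the level continuously on the navmesh.
; Whenever it is not moving, Tick picks a random navigable point within a radius of its current location and passes it to the GoToPlace event.
; GoToPlace runs AI MoveTo, setting a Moving flag while the move runs and clearing it on success or failure so the next destination gets picked.
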(event `self.ReceiveTick`
  (params (DeltaSeconds :type "Float (single-precision)"))
  (if (not (`self.Moving`))
    (bind (_randomlocation _returnvalue) (`NavigationSystemV1.K2_GetRandomLocationInNavigableRadius` (`self.K2_GetActorLocation` self) 5000.0 null null))
    (if _returnvalue
      (`self.GoToPlace` _randomlocation))))

(event `GoToPlace`
  (params (Destination :type "Vector Structure"))
  (`|AIMoveTo` self Destination null
    (:`then`
      (set `self.Moving` true))
    (:`OnSuccess`
      (set `self.Moving` false :!label _label))
    (:`OnFail`
      (goto _label))))

(fn `UserConstructionScript`)