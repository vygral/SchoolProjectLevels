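; Building system Blueprint that lets the player preview and confirm placement of buildable actors.
; While preview is on, Tick line-traces from the third-person character's follow camera, moving the preview actor to the hit point with camera yaw.
; Events toggle or cancel the preview, cycle through the PreviewActor class array, or spawn a given class.
; Confirming delegates to the preview actor's own ConfirmBuild.
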(event `SwapPreviewNext`
  (bind _returnvalue (`KismetArrayLibrary.Array_Length` (`self.PreviewActor`)))
  (if (`self.Preview`)
    (if (== _returnvalue 0)
      (`KismetSystemLibrary.PrintString` "Invalid lenght")
      (else
        (set `self.SelectedPreview` (mod (+ (`self.SelectedPreview`) 1) _returnvalue))
        (`Actor.K2_DestroyActor` (`self.PreviewBuild`))
        (bind _returnvalue_2 (`|SpawnActorFromClass` (`|GetArrayItem` (`self.PreviewActor`) (`self.SelectedPreview`)) (`KismetMathLibrary.MakeTransform` (`self.Location`)) "Undefined" "MultiplyWithRoot" null null))
        (set `self.PreviewBuild` _returnvalue_2)))))

(event `self.ReceiveBeginPlay`
  (bind _asbp_third_person_character (cast `/Game/ThirdPerson/Blueprints/BP_ThirdPersonCharacter` (`GameplayStatics.GetPlayerCharacter` 0)))
  (set `self.BP_thirdPersonCharacter` _asbp_third_person_character))

(event `ShowPreview`
  (if (> (`KismetArrayLibrary.Array_Length` (`self.PreviewActor`)) 0)
    (bind _output_get (set `self.Preview` (not (`self.Preview`))))
    (if (not _output_get)
      (`Actor.K2_DestroyActor` (`self.PreviewBuild`)))))

(event `self.ReceiveTick`
  (params (DeltaSeconds :type "Float (single-precision)"))
  (if (`self.Preview`)
    (`self.PreviewLoop`)))

(event `PreviewLoop`
  (bind (_returnvalue_location _returnvalue_rotation) (`KismetMathLibrary.BreakTransform` (`SceneComponent.K2_GetComponentToWorld` (`/Game/ThirdPerson/Blueprints/BP_ThirdPersonCharacter.FollowCamera` (`self.BP_thirdPersonCharacter`)))))
  (bind (_returnvalue_roll _returnvalue_pitch _returnvalue_yaw) (`KismetMathLibrary.BreakRotator` (`SceneComponent.K2_GetComponentRotation` (`/Game/ThirdPerson/Blueprints/BP_ThirdPersonCharacter.FollowCamera` (`self.BP_thirdPersonCharacter`)))))
  (bind (_outhit _returnvalue) (`KismetSystemLibrary.LineTraceSingle` _returnvalue_location (+ _returnvalue_location (* (`KismetMathLibrary.GetForwardVector` _returnvalue_rotation) 1000)) "TraceTypeQuery1" true (`|MakeArray` (`self.PreviewBuild`) :!type "Actor Object Reference")))
  (if _returnvalue
    (set `self.Location` (`.Location` (`GameplayStatics.BreakHitResult` _outhit))))
  (if (`KismetSystemLibrary.IsValid` (`self.PreviewBuild`))
    (`Actor.K2_SetActorLocation` (`self.PreviewBuild`) (`self.Location`) false false)
    (`Actor.K2_SetActorRotation` (`self.PreviewBuild`) (`KismetMathLibrary.MakeRotator` 0.0 0.0 _returnvalue_yaw) false)
    (else
      (bind _returnvalue_2 (`|SpawnActorFromClass` (`|GetArrayItem` (`self.PreviewActor`) (`self.SelectedPreview`)) (`KismetMathLibrary.MakeTransform` (`self.Location`) (`KismetMathLibrary.MakeRotator` 0.0)) "Undefined" "MultiplyWithRoot" null null))
      (set `self.PreviewBuild` _returnvalue_2))))

(event `ShowActorPreview`
  (params (Preview :type "/Game/MyContent/Blueprints/Building/BP_Preview Class Reference"))
  (bind _previewbuild (`self.PreviewBuild`))
  (set `self.Preview` true)
  (if (`KismetSystemLibrary.IsValid` _previewbuild)
    (`Actor.K2_DestroyActor` _previewbuild))
  (bind _returnvalue (`|SpawnActorFromClass` Preview (`KismetMathLibrary.MakeTransform` (`self.Location`)) "Undefined" "MultiplyWithRoot" null null))
  (set `self.PreviewBuild` _returnvalue))

(event `ConfirmBuild`
  (if (`self.Preview`)
    (`/Game/MyContent/Blueprints/Building/BP_Preview.ConfirmBuild` (`self.PreviewBuild`))))

(event `CancelPreview`
  (bind _previewbuild (`self.PreviewBuild`))
  (set `self.Preview` false)
  (if (`KismetSystemLibrary.IsValid` _previewbuild)
    (`Actor.K2_DestroyActor` _previewbuild)))