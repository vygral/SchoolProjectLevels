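; BP_DoorInSequence is a door that disappears once enough of its activators have been switched on in the correct order.
; EventActivatorsSwitched advances the NmbOfTrue counter only when the activating PlateTrap's index in the Activators array matches the current count.
; Reaching NmbNeeded calls Disappear, which is not defined in this graph.
; Switch-off and out-of-order activations are ignored, so progress never resets here.
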(event `self.EventActivatorsSwitched`
  (params (On :type Boolean) (PlateTrap :type "/Game/MyContent/Blueprints/SchoolTestBP/BP_PlateTrap Object Reference"))
  (if On
    (if (== (`KismetArrayLibrary.Array_Find` (`self.Activators`) PlateTrap) (`self.nmbOfTrue`))
      (bind _result (`/Engine/EditorBlueprintResources/StandardMacros.IncrementInt` (`self.nmbOfTrue`))
        (:`  `
          (if (>= _result (`self.nmbNeeded`))
            (`self.Disappear`)))))))

(fn `UserConstructionScript`
  (`parent.UserConstructionScript`))