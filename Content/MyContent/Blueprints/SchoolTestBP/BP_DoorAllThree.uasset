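; BP_DoorAllThree is a door that disappears once enough of its activators are switched on.
; Each EventActivatorsSwitched event raises or lowers the NmbOfTrue counter according to its On flag.
; When the count reaches NmbNeeded it calls Disappear, which is not defined in these graphs, and no branch here brings the door back.
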(event `self.EventActivatorsSwitched`
  (params (On :type Boolean) (PlateTrap :type "/Game/MyContent/Blueprints/SchoolTestBP/BP_PlateTrap Object Reference"))
  (bind _nmboftrue (`self.nmbOfTrue`))
  (if On
    (`/Engine/EditorBlueprintResources/StandardMacros.IncrementInt` _nmboftrue
      (:`  `
        _))
    (else
      (`/Engine/EditorBlueprintResources/StandardMacros.DecrementInt` _nmboftrue
        (:`  `
          _))))
  (if (>= _nmboftrue (`self.nmbNeeded`))
    (`self.Disappear`)))

(fn `UserConstructionScript`
  (`parent.UserConstructionScript`))