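; BP_lightChange is an interactable actor that lets the player change the color, intensity and fluctuation of an array of lights.
; PlayerInteracted opens WBP_ChangeLights with itself as TriggerActor and switches to UI-only input with a visible cursor.
; ChangeLights applies the given settings to every light in the array.
; When fluctuation is on, Tick pulses intensity between zero and the set value using a wrapped cosine timer.
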(event `self.ReceiveTick`
  (params (DeltaSeconds :type "Float (single-precision)"))
  (`parent.ReceiveTick` DeltaSeconds)
  (bind _output_get (set `self.time` (+ (`self.time`) DeltaSeconds)))
  (if (>= _output_get (* (`KismetMathLibrary.GetPI`) 2.0))
    (set `self.time` (- (`self.time`) (* (`KismetMathLibrary.GetPI`) 2.0))))
  (if (`self.LightFluctuation`)
    (for _array_element (`self.Lights`)
      (`LightComponent.SetIntensity` (`Light.LightComponent` _array_element) (* (/ (+ (`KismetMathLibrary.Cos` (`self.time`)) 1.0) 2.0) (`self.Intensity`))))))

(event `/Game/MyContent/Blueprints/SchoolTestBP/BPI_Interact.PlayerInteracted`
  (params (Player :type "/Game/ThirdPerson/Blueprints/BP_ThirdPersonCharacter Object Reference"))
  (bind _returnvalue (`GameplayStatics.GetPlayerController` 0))
  (bind _returnvalue_2 (`|CreateWidget` "/Game/MyContent/Blueprints/School_UI/WBP_ChangeLights.WBP_ChangeLights_C"))
  (set `/Game/MyContent/Blueprints/School_UI/WBP_ChangeLights.TriggerActor` self _returnvalue_2)
  (`UserWidget.AddToViewport` _returnvalue_2 0)
  (`WidgetBlueprintLibrary.SetInputMode_UIOnlyEx` _returnvalue null)
  (set `PlayerController.bShowMouseCursor` true _returnvalue))

(event `ChangeLights`
  (params (Intensity :type "Float (double-precision)") (Color :type "Color Structure") (Fluctuates :type Boolean :default false))
  (set `self.LightFluctuation` Fluctuates)
  (set `self.Intensity` Intensity)
  (for _array_element (`self.Lights`)
    (bind _lightcomponent (`Light.LightComponent` _array_element))
    (`LightComponent.SetLightColor` _lightcomponent (`KismetMathLibrary.Conv_ColorToLinearColor` Color) true)
    (`LightComponent.SetIntensity` _lightcomponent Intensity)))

(fn `UserConstructionScript`
  (`parent.UserConstructionScript`))