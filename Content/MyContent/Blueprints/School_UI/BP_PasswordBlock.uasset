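; BP_PasswordBlock is an interactable school UI actor that opens a password entry screen when the player interacts with it.
; On PlayerInteracted it creates a WBP_PasswordInput widget, hands it the actor's Password and a reference to itself as TriggerActor, and adds it to the viewport.
; It then switches the player to UI-only input and shows the mouse cursor.
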(event `/Game/MyContent/Blueprints/SchoolTestBP/BPI_Interact.PlayerInteracted`
  (params (Player :type "/Game/ThirdPerson/Blueprints/BP_ThirdPersonCharacter Object Reference"))
  (bind _returnvalue (`GameplayStatics.GetPlayerController` 0))
  (bind _returnvalue_2 (`|CreateWidget` "/Game/MyContent/Blueprints/School_UI/WBP_PasswordInput.WBP_PasswordInput_C"))
  (set `/Game/MyContent/Blueprints/School_UI/WBP_PasswordInput.Password` (`self.Password`) _returnvalue_2)
  (set `/Game/MyContent/Blueprints/School_UI/WBP_PasswordInput.TriggerActor` self _returnvalue_2)
  (`UserWidget.AddToViewport` _returnvalue_2 0)
  (`WidgetBlueprintLibrary.SetInputMode_UIOnlyEx` _returnvalue null)
  (set `PlayerController.bShowMouseCursor` true _returnvalue))

(fn `UserConstructionScript`
  (`parent.UserConstructionScript`))