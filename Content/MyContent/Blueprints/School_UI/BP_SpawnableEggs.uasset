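; BP_SpawnableEggs is an interactable egg with a survival countdown that notifies its BP_EggControler owner and destroys itself when time runs out.
; Tick drains the timer while the egg game mode is running (or absent), updating the widget's progress bar and turning it toward the camera.
; Player interaction adds time up to a maximum.
; The Show volume toggles widget visibility, while the Sphere forwards overlaps to parent logic.
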(event `self.ReceiveBeginPlay`
  (`parent.ReceiveBeginPlay`)
  (`Widget.SetVisibility` (`WidgetComponent.GetWidget` (`self.Widget`)) "Hidden")
  (set `self.time` (`self.maxTime`)))

(event `self.ReceiveTick`
  (params (DeltaSeconds :type "Float (single-precision)"))
  (bind _widget (`self.Widget`))
  (`parent.ReceiveTick` DeltaSeconds)
  (bind _asbp_third_person_game_mode_egg (cast `/Game/MyContent/Blueprints/School_UI/BP_ThirdPersonGameModeEgg` (`GameplayStatics.GetGameMode`))
    (:`then`
      (if (`/Game/MyContent/Blueprints/School_UI/BP_ThirdPersonGameModeEgg.GameRunning` _asbp_third_person_game_mode_egg)
        (bind _output_get (set `self.time` (`KismetMathLibrary.FClamp` (- (`self.time`) DeltaSeconds) 0.0 (`self.maxTime`)) :!label _label))
        (if (> _output_get 0.0)
          (bind _aswbp_egg (cast `/Game/MyContent/Blueprints/School_UI/WBP_egg` (`WidgetComponent.GetWidget` _widget)))
          (`SceneComponent.K2_SetWorldRotation` (`self.Widget`) (`KismetMathLibrary.FindLookAtRotation` (`SceneComponent.K2_GetComponentLocation` _widget) (`SceneComponent.K2_GetComponentLocation` (`PlayerCameraManager.TransformComponent` (`GameplayStatics.GetPlayerCameraManager` 0)))) false false)
          (`ProgressBar.SetPercent` (`/Game/MyContent/Blueprints/School_UI/WBP_egg.ProgressBar_135` _aswbp_egg) (`KismetMathLibrary.FClamp` (/ (`self.time`) (`self.maxTime`))))
          (else
            (bind _asbp_egg_controler (cast `/Game/MyContent/Blueprints/School_UI/BP_EggControler` (`self.GetOwner`)))
            (`/Game/MyContent/Blueprints/School_UI/BP_EggControler.EggsDied` _asbp_egg_controler)
            (`self.K2_DestroyActor`)))))
    (:`CastFailed`
      (goto _label))))

(event `self.Show.OnComponentBeginOverlap`
  (params (OverlappedComponent :type "PrimitiveComponent Object Reference") (OtherActor :type "Actor Object Reference") (OtherComp :type "PrimitiveComponent Object Reference") (OtherBodyIndex :type Integer) (bFromSweep :type Boolean) (SweepResult :type "HitResult Structure (by ref)"))
  (cast `/Game/ThirdPerson/Blueprints/BP_ThirdPersonCharacter` OtherActor)
  (`Widget.SetVisibility` (`WidgetComponent.GetWidget` (`self.Widget`)) "Visible"))

(event `self.Sphere.OnComponentBeginOverlap`
  (params (OverlappedComponent :type "PrimitiveComponent Object Reference") (OtherActor :type "Actor Object Reference") (OtherComp :type "PrimitiveComponent Object Reference") (OtherBodyIndex :type Integer) (bFromSweep :type Boolean) (SweepResult :type "HitResult Structure (by ref)"))
  (`parent.ReceiveActorBeginOverlap` OtherActor))

(event `self.Show.OnComponentEndOverlap`
  (params (OverlappedComponent :type "PrimitiveComponent Object Reference") (OtherActor :type "Actor Object Reference") (OtherComp :type "PrimitiveComponent Object Reference") (OtherBodyIndex :type Integer))
  (bind _returnvalue (`WidgetComponent.GetWidget` (`self.Widget`)))
  (cast `/Game/ThirdPerson/Blueprints/BP_ThirdPersonCharacter` OtherActor)
  (if (`KismetSystemLibrary.IsValid` _returnvalue)
    (`Widget.SetVisibility` _returnvalue "Hidden")))

(event `self.Sphere.OnComponentEndOverlap`
  (params (OverlappedComponent :type "PrimitiveComponent Object Reference") (OtherActor :type "Actor Object Reference") (OtherComp :type "PrimitiveComponent Object Reference") (OtherBodyIndex :type Integer))
  (`parent.ReceiveActorEndOverlap` OtherActor))

(event `self.PlayerInteracted`
  (params (Player :type "/Game/ThirdPerson/Blueprints/BP_ThirdPersonCharacter Object Reference"))
  (set `self.time` (`KismetMathLibrary.FClamp` (+ (`self.time`) (`self.TimeAdded`)) 0.0 (`self.maxTime`))))

(event `self.ReceiveActorBeginOverlap`
  (params (OtherActor :type "Actor Object Reference")))

(event `self.ReceiveActorEndOverlap`
  (params (OtherActor :type "Actor Object Reference")))

(fn `UserConstructionScript`
  (`parent.UserConstructionScript`))