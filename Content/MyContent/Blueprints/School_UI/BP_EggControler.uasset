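; Egg controller for an egg minigame that spawns timed eggs inside its SpawningRange box and tells the egg game mode when the game ends.
; On the game mode's GameStarted event, GeneratePositions builds a 100-unit grid of candidates and randomly picks spots without repeats.
; Difficulty raises the egg count and shortens each spawned egg's timer and added time.
; EggsDied calls GameEnded on the game mode.
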(event `EggsDied`
  (bind _asbp_third_person_game_mode_egg (cast `/Game/MyContent/Blueprints/School_UI/BP_ThirdPersonGameModeEgg` (`GameplayStatics.GetGameMode`)))
  (`/Game/MyContent/Blueprints/School_UI/BP_ThirdPersonGameModeEgg.GameEnded` _asbp_third_person_game_mode_egg))

(event `self.ReceiveBeginPlay`
  (bind _asbp_third_person_game_mode_egg (cast `/Game/MyContent/Blueprints/School_UI/BP_ThirdPersonGameModeEgg` (`GameplayStatics.GetGameMode`)))
  (add `/Game/MyContent/Blueprints/School_UI/BP_ThirdPersonGameModeEgg.GameStarted` _asbp_third_person_game_mode_egg (delegate `GameStarted`)))

(event `GameStarted`
  (bind _spawningrange (`self.SpawningRange`))
  (bind (_returnvalue_x _returnvalue_y _returnvalue_z) (`KismetMathLibrary.BreakVector` (`BoxComponent.GetScaledBoxExtent` _spawningrange)))
  (bind (_returnvalue_x_2 _returnvalue_y_2 _returnvalue_z_2) (`KismetMathLibrary.BreakVector` (`SceneComponent.K2_GetComponentLocation` _spawningrange)))
  (bind _asbp_third_person_game_mode_egg (cast `/Game/MyContent/Blueprints/School_UI/BP_ThirdPersonGameModeEgg` (`GameplayStatics.GetGameMode`)))
  (bind _difficulty (`/Game/MyContent/Blueprints/School_UI/BP_ThirdPersonGameModeEgg.Difficulty` _asbp_third_person_game_mode_egg))
  (bind _locations (`self.GeneratePositions` (+ (* _difficulty 4.0) 3)))
  (for _array_element _locations
    (bind _returnvalue (`KismetMathLibrary.MakeVector` (+ (`KismetMathLibrary.BreakVector2D` _array_element) _returnvalue_x_2) (+ (`.Y` (`KismetMathLibrary.BreakVector2D` _array_element)) _returnvalue_y_2) (- _returnvalue_z_2 _returnvalue_z)))
    (`KismetSystemLibrary.PrintString` (`KismetStringLibrary.Conv_VectorToString` _returnvalue))
    (bind _returnvalue_2 (`|SpawnActorFromClass` "/Game/MyContent/Blueprints/School_UI/BP_SpawnableEggs.BP_SpawnableEggs_C" (`KismetMathLibrary.MakeTransform` _returnvalue) "Undefined" "MultiplyWithRoot" self null))
    (bind _returnvalue_3 (- 20.0 (* _difficulty 15.0)))
    (set `/Game/MyContent/Blueprints/School_UI/BP_SpawnableEggs.maxTime` _returnvalue_3 _returnvalue_2)
    (set `/Game/MyContent/Blueprints/School_UI/BP_SpawnableEggs.time` _returnvalue_3 _returnvalue_2)
    (set `/Game/MyContent/Blueprints/School_UI/BP_SpawnableEggs.TimeAdded` (- 5.0 (* _difficulty 3.0)) _returnvalue_2)))

(fn `GeneratePositions`
  (params (NumberOfLocations :type Integer))
  (returns (Locations :type "Array of Vector2D Structure"))
  (locals (PossibleLocations :type "Array of Vector2D Structure") (FinalLocations :type "Array of Vector2D Structure") (RandomNumber :type Integer))
  (bind _spawningrange (`self.SpawningRange`))
  (bind _possiblelocations (`local.PossibleLocations`))
  (bind (_returnvalue_x _returnvalue_y) (`KismetMathLibrary.BreakVector` (`BoxComponent.GetScaledBoxExtent` (`self.SpawningRange`))))
  (bind (_returnvalue_x_2 _returnvalue_y_2) (`KismetMathLibrary.BreakVector` (`BoxComponent.GetScaledBoxExtent` _spawningrange)))
  (bind (_returnvalue_x_3 _returnvalue_y_3) (`KismetMathLibrary.BreakVector` (`SceneComponent.K2_GetComponentLocation` _spawningrange)))
  (for _index (range 1 (+ (/ (`KismetMathLibrary.FTrunc` (`KismetMathLibrary.Abs` (- _returnvalue_x_3 (* _returnvalue_x_2 2.0)))) 100) 1))
    (for _index_2 (range 1 (+ (/ (`KismetMathLibrary.FTrunc` (`KismetMathLibrary.Abs` (- _returnvalue_y_3 (* _returnvalue_y_2 2.0)))) 100) 1))
      (`KismetArrayLibrary.Array_Add` (`local.PossibleLocations`) (`KismetMathLibrary.MakeVector2D` (- (`KismetMathLibrary.Conv_IntToDouble` (* _index 100)) _returnvalue_x) (- (`KismetMathLibrary.Conv_IntToDouble` (* _index_2 100)) _returnvalue_y)))))
  (if (> (`KismetArrayLibrary.Array_Length` (`local.PossibleLocations`)) (`local.NumberOfLocations`))
    (for _ (range (+ (`local.NumberOfLocations`) 1))
      (bind _output_get (set `local.RandomNumber` (`KismetMathLibrary.RandomInteger` (`KismetArrayLibrary.Array_Length` _possiblelocations))))
      (`KismetArrayLibrary.Array_Add` (`local.FinalLocations`) (`|GetArrayItem` _possiblelocations _output_get))
      (`KismetArrayLibrary.Array_Remove` _possiblelocations _output_get))
    (else
      (`KismetSystemLibrary.PrintString` "Not enough space")))
  (return (`local.FinalLocations`)))

(fn `UserConstructionScript`)