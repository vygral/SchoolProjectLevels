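; BP_Reactor2 is a reactor actor that shuts off its sphere once enough linked trigger plates have fired.
; On BeginPlay it binds to each plate's event dispatcher in the TriggerPlate array.
; Each triggered plate gets a new cube material, has its dispatcher unbound and increments a press counter.
; When the counter reaches RequiredPressed, the sphere is hidden and its collision disabled, with debug prints along the way.
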(event `self.ReceiveBeginPlay`
  (for _array_element (`self.TriggerPlate`)
    (add `/Game/MyContent/Blueprints/School_BP/BP_triggerPlate.EventDispatcher1` _array_element (delegate `PlateTriggered`))))

(event `PlateTriggered`
  (params (BP_triggerPlate :type "/Game/MyContent/Blueprints/School_BP/BP_triggerPlate Object Reference"))
  (bind _asbp_trigger_plate (cast `/Game/MyContent/Blueprints/School_BP/BP_triggerPlate` BP_triggerPlate))
  (`PrimitiveComponent.SetMaterial` (`/Game/MyContent/Blueprints/School_BP/BP_triggerPlate.Cube` BP_triggerPlate) 0 "/Game/MyContent/Materials/M_BaseMaterial.M_BaseMaterial")
  (clear `/Game/MyContent/Blueprints/School_BP/BP_triggerPlate.EventDispatcher1` _asbp_trigger_plate)
  (`KismetSystemLibrary.PrintString` "Hello")
  (bind _result (`/Engine/EditorBlueprintResources/StandardMacros.IncrementInt` (`self.pressedNmb`))
    (:`  `
      (if (>= _result (`self.requiredPressed`))
        (`KismetSystemLibrary.PrintString` "Reactor is triggered")
        (`SceneComponent.SetVisibility` (`self.Sphere`) false false)
        (`PrimitiveComponent.SetCollisionEnabled` (`self.Sphere`) "NoCollision")))))

(fn `UserConstructionScript`)