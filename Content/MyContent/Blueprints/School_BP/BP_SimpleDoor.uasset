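; Puzzle door that moves a straight wall vertically once all of its linked light switches are on.
; It binds to each switch's finished event and tracks their states in a bool array.
; With InOrder set, switch-ons only count in array order, and switching one off can roll the progress index back.
; A timeline scaled by MoveZ plays when all states are true and reverses otherwise.
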(event `self.ReceiveBeginPlay`
  (for _array_element (`self.BP_lightSwitch`)
    (add `/Game/MyContent/Blueprints/School_BP/BP_LightSwitch.SwitchFinished` _array_element (delegate `SwitchFinished`))
    (`KismetArrayLibrary.Array_Add` (`self.AreOn`))))

(event `SwitchFinished`
  (params (IsOn :type Boolean) (BP_LightSwitch :type "/Game/MyContent/Blueprints/School_BP/BP_LightSwitch Object Reference"))
  (bind _returnvalue (`KismetArrayLibrary.Array_Find` (`self.BP_lightSwitch`) BP_LightSwitch))
  (if (and IsOn (`self.InOrder`))
    (if (== BP_LightSwitch (`|GetArrayItem` (`self.BP_lightSwitch`) (`self.NmbOrder`)))
      (`/Engine/EditorBlueprintResources/StandardMacros.IncrementInt` (`self.NmbOrder`)
        (:`  `
          (`KismetArrayLibrary.Array_Set` (`self.AreOn`) _returnvalue IsOn :!label _label)
          (if (`KismetArrayLibrary.Array_Contains` (`self.AreOn`))
            (bind (_direction _floattrack) (`Timeline|Timeline` :!via `Reverse` :!label _label_2)
              (:`Update`
                (`SceneComponent.K2_SetRelativeLocation` (`self.SM_2StraightWall`) (`KismetMathLibrary.MakeVector` 0.0 0.0 (* _floattrack (`self.MoveZ`))) false false)))
            (else
              (goto _label_2))))))
    (elif (<= _returnvalue (`self.NmbOrder`))
      (set `self.NmbOrder` _returnvalue)
      (goto _label)
      (else
        (goto _label)))))

(fn `UserConstructionScript`)