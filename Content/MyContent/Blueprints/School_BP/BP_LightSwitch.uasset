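; BP_LightSwitch is an interactable light switch that notifies BP_ThirdPersonCharacter when it enters or leaves the switch's overlap area, passing itself along.
; EventSwitch uses a FlipFlop to alternately play and reverse a timeline that rolls the LightSwitchPart2 component.
; When the timeline finishes, it stores the FlipFlop state in IsOn and broadcasts SwitchFinished with that state and itself.
; SwitchOff is an empty event.
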(event `self.ReceiveBeginPlay`)

(event `EventSwitch`
  (bind _isa (`/Engine/EditorBlueprintResources/StandardMacros.FlipFlop`)
    (:`A`
      (bind (_direction _floattrack) (`Timeline|Timeline` :!label _label)
        (:`Update`
          (`SceneComponent.K2_SetRelativeRotation` (`self.LightSwitchPart2`) (`KismetMathLibrary.MakeRotator` (* _floattrack 10.0)) false false))
        (:`Finished`
          (bind _output_get (set `self.IsOn` _isa))
          (`self.SwitchFinished` _output_get self))))
    (:`B`
      (goto _label :!via `Reverse`))))

(event `self.ReceiveActorBeginOverlap`
  (params (OtherActor :type "Actor Object Reference"))
  (bind _asbp_third_person_character (cast `/Game/ThirdPerson/Blueprints/BP_ThirdPersonCharacter` OtherActor))
  (`/Game/ThirdPerson/Blueprints/BP_ThirdPersonCharacter.EventInLightSwitchRadius` _asbp_third_person_character self))

(event `self.ReceiveActorEndOverlap`
  (params (OtherActor :type "Actor Object Reference"))
  (bind _asbp_third_person_character (cast `/Game/ThirdPerson/Blueprints/BP_ThirdPersonCharacter` OtherActor))
  (`/Game/ThirdPerson/Blueprints/BP_ThirdPersonCharacter.EventOutLightSwitchRadius` _asbp_third_person_character self))

(event `SwitchOff`)

(fn `UserConstructionScript`)