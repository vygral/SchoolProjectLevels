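; BP_Reactor is a sequence puzzle actor that shuts off its sphere once five trigger plates are activated in array order.
; On BeginPlay it binds PlateTriggered to every plate's event dispatcher.
; Only the plate matching the current PressedNmb index advances the count, changing its cube material and unbinding; out-of-order plates are ignored without a reset.
; At five, the sphere is hidden and its collision disabled.
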(event `self.ReceiveBeginPlay`
  (for _array_element (`self.TriggerPlate`)
    (add `/Game/MyContent/Blueprints/School_BP/BP_triggerPlate.EventDispatcher1` _array_element (delegate `PlateTriggered`))))

(event `PlateTriggered`
  (params (BP_triggerPlate :type "/Game/MyContent/Blueprints/School_BP/BP_triggerPlate Object Reference"))
  (bind _pressednmb (`self.pressedNmb`))
  (bind _output (`|GetArrayItem` (`self.TriggerPlate`) _pressednmb))
  (if (== BP_triggerPlate _output)
    (`PrimitiveComponent.SetMaterial` (`/Game/MyContent/Blueprints/School_BP/BP_triggerPlate.Cube` _output) 0 "/Game/MyContent/Materials/M_BaseMaterial.M_BaseMaterial")
    (clear `/Game/MyContent/Blueprints/School_BP/BP_triggerPlate.EventDispatcher1` _output)
    (`KismetSystemLibrary.PrintString` "Hello")
    (bind _result (`/Engine/EditorBlueprintResources/StandardMacros.IncrementInt` _pressednmb)
      (:`  `
        (if (>= _result 5)
          (`KismetSystemLibrary.PrintString` "Reactor is triggered")
          (`SceneComponent.SetVisibility` (`self.Sphere`) false false)
          (`PrimitiveComponent.SetCollisionEnabled` (`self.Sphere`) "NoCollision"))))))

(fn `UserConstructionScript`)