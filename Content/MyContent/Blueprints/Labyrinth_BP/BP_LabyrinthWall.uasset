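; Labyrinth wall actor Blueprint, apparently meant to build one maze cell from four directional wall flags.
; An unconnected node chain adds a base static mesh component, then one offset along X or Y for each set flag, all using SM_0Wall.
; The ChooseWall event takes the four flags but has an empty body, and the construction script is empty, so the actor currently builds nothing.
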(event `ChooseWall`
  (params (rightWall :type Boolean) (topWall :type Boolean) (leftWall :type Boolean) (bottomWall :type Boolean)))

(fn `UserConstructionScript`)