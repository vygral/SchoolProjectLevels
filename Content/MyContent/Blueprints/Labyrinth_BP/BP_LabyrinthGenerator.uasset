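; Labyrinth generator actor that builds a random grid maze from wall, floor and end-marker actors when GenerateWalls runs, destroying the previous layout first.
; SelectWalls carves a random walk from an edge cell until stuck, placing the end there, then CreateSidePaths opens random eligible cells until none remain.
; CanMove allows carving only interior walls with exactly one open orthogonal neighbour, so paths branch without forming loops.
; Nothing in this graph triggers generation; BeginPlay is empty.
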(event `self.ReceiveBeginPlay`)

(event `GenerateWalls`
  (bind (_returnvalue_x _returnvalue_y _returnvalue_z) (`KismetMathLibrary.BreakVector` (`self.K2_GetActorLocation`)))
  (bind (_returnvalue_x_2 _returnvalue_y_2 _returnvalue_z_2) (`KismetMathLibrary.BreakVector` (`self.K2_GetActorLocation`)))
  (bind _sizex (`self.SizeX`))
  (for _array_element (`self.Labyrinth`)
    (`self.K2_DestroyActor` _array_element))
  (`KismetArrayLibrary.Array_Clear` (`self.Labyrinth`))
  (bind (_walls _endposx _endposy) (`self.SelectWalls` (`self.SizeX`) (`self.SizeY`) 2))
  (bind _returnvalue (`|SpawnActorFromClass` (`self.EndObject`) (`KismetMathLibrary.MakeTransform` (`KismetMathLibrary.MakeVector` (+ _returnvalue_x (* _endposx 300)) (+ _returnvalue_y (* _endposy 300)) _returnvalue_z)) "Undefined" "MultiplyWithRoot" null null))
  (`KismetArrayLibrary.Array_Add` (`self.Labyrinth`) _returnvalue)
  (bind _output_get (set `self.Walls` _walls))
  (for (_array_element_2 _array_index) _output_get
    (if _array_element_2
      (bind _returnvalue_2 (+ (`KismetMathLibrary.Conv_IntToDouble` (* (mod _array_index _sizex) 300)) _returnvalue_x_2))
      (bind _returnvalue_3 (+ (`KismetMathLibrary.Conv_IntToDouble` (* (/ _array_index _sizex) 300)) _returnvalue_y_2))
      (bind _returnvalue_4 (`|SpawnActorFromClass` (`self.WallObject`) (`KismetMathLibrary.MakeTransform` (`KismetMathLibrary.MakeVector` _returnvalue_2 _returnvalue_3 _returnvalue_z_2)) "Undefined" "MultiplyWithRoot" null null))
      (`KismetArrayLibrary.Array_Add` (`self.Labyrinth`) _returnvalue_4)
      (else
        (bind _returnvalue_5 (`|SpawnActorFromClass` (`self.NonWallObject`) (`KismetMathLibrary.MakeTransform` (`KismetMathLibrary.MakeVector` _returnvalue_2 _returnvalue_3 _returnvalue_z_2)) "Undefined" "MultiplyWithRoot" null null))
        (`KismetArrayLibrary.Array_Add` (`self.Labyrinth`) _returnvalue_5)))))

(fn `CanMove`
  (params (Walls :type "Array of Boolean") (LocationX :type Integer) (LocationY :type Integer) (SizeX :type Integer) (SizeY :type Integer))
  (returns (Can :type Boolean))
  (locals (getOut :type Boolean))
  (if (or (<= LocationX 0) (<= LocationY 0) (>= LocationX (- SizeX 1)) (>= LocationY (- SizeY 1)))
    (return false)
    (else
      (bind _iswall (`self.IsWall` (`local.Walls`) (`local.LocationX`) (`local.LocationY`) (`local.SizeX`) (`local.SizeY`)))
      (set `local.getOut` (not _iswall))
      (bind _iswall_2 (`self.IsWall` (`local.Walls`) (`local.LocationX`) (- (`local.LocationY`) 1) (`local.SizeX`) (`local.SizeY`)))
      (if (not _iswall_2)
        (if (not (stale _output_get))
          (bind _output_get (set `local.getOut` true))
          (bind _iswall_3 (`self.IsWall` (`local.Walls`) (- (`local.LocationX`) 1) (`local.LocationY`) (`local.SizeX`) (`local.SizeY`) :!label _label))
          (if (not _iswall_3)
            (if (not (stale _output_get_2))
              (bind _output_get_2 (set `local.getOut` true))
              (bind _iswall_4 (`self.IsWall` (`local.Walls`) (+ (`local.LocationX`) 1) (`local.LocationY`) (`local.SizeX`) (`local.SizeY`) :!label _label_2))
              (if (not _iswall_4)
                (if (not (stale _output_get_3))
                  (bind _output_get_3 (set `local.getOut` true))
                  (bind _iswall_5 (`self.IsWall` (`local.Walls`) (`local.LocationX`) (+ (`local.LocationY`) 1) (`local.SizeX`) (`local.SizeY`) :!label _label_3))
                  (if (not _iswall_5)
                    (if (stale _output_get_4)
                      _
                      (else
                        (bind _output_get_4 (set `local.getOut` true))
                        (return true)))
                    (elif (`local.getOut`)
                      (return true)
                      (else
                        (return false)))))
                (else
                  (goto _label_3))))
            (else
              (goto _label_2))))
        (else
          (goto _label)))
      (return false))))

(fn `CreateSidePaths`
  (params (LWalls :type "Array of Boolean"))
  (returns (LWallsOut :type "Array of Boolean"))
  (locals (PosibleMoves :type "Array of Integer"))
  (bind _returnvalue (`KismetArrayLibrary.Array_Length` (`local.PosibleMoves`)))
  (for (_ _array_index) (`local.LWalls`) :!label _label
    (bind _can (`self.CanMove` (`local.LWalls`) (mod _array_index (`self.SizeX`)) (/ _array_index (`self.SizeX`)) (`self.SizeX`) (`self.SizeY`)))
    (if _can
      (`KismetArrayLibrary.Array_Add` (`local.PosibleMoves`) _array_index)))
  (while (> _returnvalue 0)
    (`KismetArrayLibrary.Array_Set` (`local.LWalls`) (`|GetArrayItem` (`local.PosibleMoves`) (`KismetMathLibrary.RandomInteger` _returnvalue)))
    (`KismetArrayLibrary.Array_Clear` (`local.PosibleMoves`))
    (goto _label))
  (return (`local.LWalls`)))

(fn `GetMove`
  (params (Walls :type "Array of Boolean") (PositionX :type Integer) (PositionY :type Integer) (SizeX :type Integer) (SizeY :type Integer))
  (returns (Walls_out :type "Array of Boolean") (newPositionX :type Integer) (newPositionY :type Integer) (NoMoves :type Boolean))
  (locals (NumberOfPossibleMoves :type Integer) (Moves :type "Array of Vector2D Structure") (RandomNumber :type Integer))
  (bind _returnvalue (<= (`local.NumberOfPossibleMoves`) 0))
  (bind _can (`self.CanMove` (`local.Walls`) (- (`local.PositionX`) 1) (`local.PositionY`) (`local.SizeX`) (`local.SizeY`)))
  (if _can
    (`KismetArrayLibrary.Array_Add` (`local.Moves`) (-1.0 0.0))
    (set `local.NumberOfPossibleMoves` (+ (`local.NumberOfPossibleMoves`) 1)))
  (bind _can_2 (`self.CanMove` (`local.Walls`) (+ (`local.PositionX`) 1) (`local.PositionY`) (`local.SizeX`) (`local.SizeY`)))
  (if _can_2
    (`KismetArrayLibrary.Array_Add` (`local.Moves`) (1.0 0.0))
    (set `local.NumberOfPossibleMoves` (+ (`local.NumberOfPossibleMoves`) 1)))
  (bind _can_3 (`self.CanMove` (`local.Walls`) (`local.PositionX`) (- (`local.PositionY`) 1) (`local.SizeX`) (`local.SizeY`)))
  (if _can_3
    (`KismetArrayLibrary.Array_Add` (`local.Moves`) (0.0 -1.0))
    (set `local.NumberOfPossibleMoves` (+ (`local.NumberOfPossibleMoves`) 1)))
  (bind _can_4 (`self.CanMove` (`local.Walls`) (`local.PositionX`) (+ (`local.PositionY`) 1) (`local.SizeX`) (`local.SizeY`)))
  (if _can_4
    (`KismetArrayLibrary.Array_Add` (`local.Moves`) (0.0 1.0))
    (set `local.NumberOfPossibleMoves` (+ (`local.NumberOfPossibleMoves`) 1)))
  (if _returnvalue
    (return (`local.Walls`) (`local.PositionX`) (`local.PositionY`) _returnvalue)
    (else
      (bind _output_get (set `local.RandomNumber` (`KismetMathLibrary.RandomInteger` (`local.NumberOfPossibleMoves`))))
      (bind (_returnvalue_x _returnvalue_y) (`KismetMathLibrary.BreakVector2D` (`KismetMathLibrary.ToRounded2D` (`|GetArrayItem` (`local.Moves`) _output_get))))
      (bind _returnvalue_2 (+ (`local.PositionX`) _returnvalue_x))
      (bind _returnvalue_3 (+ _returnvalue_y (`local.PositionY`)))
      (bind _returnvalue_4 (+ _returnvalue_2 (* (`local.SizeX`) _returnvalue_3)))
      (`KismetSystemLibrary.PrintString` (`KismetStringLibrary.Concat_StrStr` "The index: " (`KismetStringLibrary.Conv_IntToString` _returnvalue_4)) false true (struct :`G` 0.66 :`B` 1.0 :`A` 1.0) 300.0)
      (`KismetArrayLibrary.Array_Set` (`local.Walls`) _returnvalue_4)
      (return (`local.Walls`) _returnvalue_2 _returnvalue_3 false))))

(fn `GetNeigboringWalls`
  (params (LocationX :type Integer) (LocationY :type Integer) (SizeX :type Integer) (SizeY :type Integer))
  (returns (RightWall :type Boolean) (TopWall :type Boolean) (LeftWall :type Boolean) (BottomWall :type Boolean))
  (bind _iswall (`self.IsWall` (`self.Walls`) (`local.LocationX`) (- (`local.LocationY`) 1) (`self.SizeX`) (`self.SizeY`)))
  (bind _iswall_2 (`self.IsWall` (`self.Walls`) (- (`local.LocationX`) 1) (`local.LocationY`) (`self.SizeX`) (`self.SizeY`)))
  (bind _iswall_3 (`self.IsWall` (`self.Walls`) (+ (`local.LocationX`) 1) (`local.LocationY`) (`self.SizeX`) (`self.SizeY`)))
  (bind _iswall_4 (`self.IsWall` (`self.Walls`) (`local.LocationX`) (+ (`local.LocationY`) 1) (`self.SizeX`) (`self.SizeY`)))
  (return _iswall_3 _iswall_4 _iswall_2 _iswall))

(fn `IsWall`
  (params (Walls :type "Array of Boolean") (x :type Integer) (y :type Integer) (sizeX :type Integer) (sizeY :type Integer))
  (returns (isWall :type Boolean))
  (if (or (< x 0) (>= x sizeX) (>= y sizeY) (< y 0))
    (return false)
    (else
      (return (`|GetArrayItem` (`local.Walls`) (+ x (* y sizeX)))))))

(fn `SelectWalls`
  (params (SizeX :type Integer) (SizeY :type Integer) (StartX :type Integer))
  (returns (Walls :type "Array of Boolean") (EndPosX :type Integer) (EndPosY :type Integer))
  (locals (lWalls :type "Array of Boolean") (lCurrentPosition :type "Array of Integer"))
  (bind _lcurrentposition (`local.lCurrentPosition`))
  (bind _lcurrentposition_2 (`local.lCurrentPosition`))
  (set `local.lCurrentPosition` (`|MakeArray` StartX 0))
  (for _ (range (`local.SizeY`))
    (for _ (range (`local.SizeX`))
      (`KismetArrayLibrary.Array_Add` (`local.lWalls`) true)))
  (`KismetArrayLibrary.Array_Set` (`local.lWalls`) (`local.StartX`))
  (bind (_walls_out _newpositionx _newpositiony _nomoves) (`self.GetMove` (`local.lWalls`) (`|GetArrayItem` _lcurrentposition) (`|GetArrayItem` _lcurrentposition 1) (`local.SizeX`) (`local.SizeY`) :!label _label))
  (`KismetSystemLibrary.PrintString` (`KismetStringLibrary.Concat_StrStr` (`KismetStringLibrary.Conv_IntToString` _newpositionx) "  " (`KismetStringLibrary.Conv_IntToString` _newpositiony)) false true (struct :`G` 0.66 :`B` 1.0 :`A` 1.0) 3.0)
  (while (not _nomoves)
    (set `local.lWalls` _walls_out)
    (`KismetArrayLibrary.Array_Set` _lcurrentposition_2 0 _newpositionx)
    (`KismetArrayLibrary.Array_Set` _lcurrentposition_2 1 _newpositiony)
    (goto _label))
  (bind _lwallsout (`self.CreateSidePaths` (`local.lWalls`)))
  (bind _output_get (set `local.lWalls` _lwallsout))
  (return _output_get _newpositionx _newpositiony))

(fn `UserConstructionScript`)