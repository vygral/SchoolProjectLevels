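; BP_SpikePoint is a rotating spike actor that changes the score when the player pawn overlaps it.
; On overlap it adds PointsDif to Points on the BP_Scoring game mode, clamps the result at zero, then destroys itself.
; Tick yaws the Spike component by RotationSpeed scaled with delta time.
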(event `self.ReceiveActorBeginOverlap`
  (params (OtherActor :type "Actor Object Reference"))
  (if (== OtherActor (`GameplayStatics.GetPlayerPawn` 0))
    (bind _asbp_scoring (cast `/Game/MyContent/Blueprints/BP_Scoring` (`GameplayStatics.GetGameMode`))
      (:`then`
        (bind _returnvalue (+ (`/Game/MyContent/Blueprints/BP_Scoring.Points` _asbp_scoring) (`self.PointsDif`)))
        (if (>= _returnvalue 0)
          (set `/Game/MyContent/Blueprints/BP_Scoring.Points` _returnvalue _asbp_scoring)
          (else
            (set `/Game/MyContent/Blueprints/BP_Scoring.Points` 0 _asbp_scoring)))
        (`self.K2_DestroyActor`))
      (:`CastFailed`
        (`KismetSystemLibrary.PrintString` "CastFailed")))))

(event `self.ReceiveTick`
  (params (DeltaSeconds :type "Float (single-precision)"))
  (`SceneComponent.K2_AddLocalRotation` (`self.spike`) (`KismetMathLibrary.MakeRotator` 0.0 0.0 (* DeltaSeconds (`self.RotationSpeed`))) false false))

(fn `UserConstructionScript`)