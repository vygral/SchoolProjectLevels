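; BP_pinballAddPoints1 is a pinball bumper that awards points and kicks back the ball when hit.
; A hit on the Valec component by a BP_PinballBall calls AddPoints with PointToAdd on the parent BP_PinBallGame actor, then fires a RadialForce impulse.
; It relies on being a child actor of the game, since nothing happens without that parent.
; A leftover ActorBeginOverlap event only prints a debug string.
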(event `self.ReceiveActorBeginOverlap`
  (params (OtherActor :type "Actor Object Reference"))
  (`KismetSystemLibrary.PrintString` "Hello"))

(event `self.valec.OnComponentHit`
  (params (HitComponent :type "PrimitiveComponent Object Reference") (OtherActor :type "Actor Object Reference") (OtherComp :type "PrimitiveComponent Object Reference") (NormalImpulse :type "Vector Structure") (Hit :type "HitResult Structure (by ref)"))
  (bind _returnvalue (`self.GetParentActor`))
  (cast `/Game/MyContent/Blueprints/Pinball/BP_PinballBall` OtherActor)
  (if (`KismetSystemLibrary.IsValid` _returnvalue)
    (bind _asbp_pin_ball_game (cast `/Game/MyContent/Blueprints/Pinball/BP_PinBallGame` _returnvalue))
    (`/Game/MyContent/Blueprints/Pinball/BP_PinBallGame.AddPoints` _asbp_pin_ball_game (`self.pointToAdd`))
    (`RadialForceComponent.FireImpulse` (`self.RadialForce`))))

(fn `UserConstructionScript`)