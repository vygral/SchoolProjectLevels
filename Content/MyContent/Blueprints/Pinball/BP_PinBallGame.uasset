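; Pinball table actor that runs the flippers, scoring, ball respawn and a saved high score.
; F and G drive timelines that rotate the left and right flippers, reversing on release.
; A drain box destroys the ball, respawns one through a child-actor spawner and resets points.
; AddPoints updates the text and saves via BP_PinballSave when HighScore is beaten, though HighScore is never set to Points.
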(event `self.ReceiveBeginPlay`
  (bind _asbp_pinball_spawner (cast `/Game/MyContent/Blueprints/Pinball/BP_pinballSpawner` (`ChildActorComponent.ChildActor` (`self.BP_pinballSpawner`))))
  (`/Game/MyContent/Blueprints/Pinball/BP_pinballSpawner.SpawnBall` _asbp_pinball_spawner)
  (`self.load`)
  (`TextRenderComponent.K2_SetText` (`self.TextRender`) (`KismetTextLibrary.Conv_IntToText` (`self.HighScore`))))

(event `Key|F`
  (params (Key :type "Key Structure"))
  (:`Pressed`
    (bind (_direction _controlleftrotation) (`Timeline|ControlLeft` :!label _label)
      (:`Update`
        (`SceneComponent.K2_SetRelativeRotation` (`self.packa1`) (`KismetMathLibrary.MakeRotator` 0.0 0.0 (* _controlleftrotation (`self.rotationUpDown`))) false false))))
  (:`Released`
    (goto _label :!via `Reverse`)))

(event `Key|G`
  (params (Key :type "Key Structure"))
  (:`Pressed`
    (bind (_direction _controlrightrotation) (`Timeline|ControlRight` :!label _label_2)
      (:`Update`
        (`SceneComponent.K2_SetRelativeRotation` (`self.packa2`) (`KismetMathLibrary.MakeRotator` 0.0 0.0 (* _controlrightrotation (`self.rotationUpDown`))) false false))))
  (:`Released`
    (goto _label_2 :!via `Reverse`)))

(event `AddPoints`
  (params (PointsToAdd :type Integer))
  (bind _output_get (set `self.Points` (+ PointsToAdd (`self.Points`))))
  (`TextRenderComponent.K2_SetText` (`self.TextRender`) (`KismetTextLibrary.Conv_IntToText` _output_get))
  (if (< (`self.HighScore`) (`self.Points`))
    (`self.Save`)))

(event `self.Box.OnComponentBeginOverlap`
  (params (OverlappedComponent :type "PrimitiveComponent Object Reference") (OtherActor :type "Actor Object Reference") (OtherComp :type "PrimitiveComponent Object Reference") (OtherBodyIndex :type Integer) (bFromSweep :type Boolean) (SweepResult :type "HitResult Structure (by ref)"))
  (bind _asbp_pinball_ball (cast `/Game/MyContent/Blueprints/Pinball/BP_PinballBall` OtherActor))
  (`self.K2_DestroyActor` _asbp_pinball_ball)
  (bind _asbp_pinball_spawner (cast `/Game/MyContent/Blueprints/Pinball/BP_pinballSpawner` (`ChildActorComponent.ChildActor` (`self.BP_pinballSpawner`))))
  (`/Game/MyContent/Blueprints/Pinball/BP_pinballSpawner.SpawnBall` _asbp_pinball_spawner)
  (bind _output_get (set `self.Points` 0))
  (`TextRenderComponent.K2_SetText` (`self.TextRender`) (`KismetTextLibrary.Conv_IntToText` _output_get))
  (`TextRenderComponent.K2_SetText` (`self.TextRender`) (`KismetTextLibrary.Conv_IntToText` (`self.HighScore`))))

(fn `load`
  (bind _returnvalue (`GameplayStatics.DoesSaveGameExist` (`self.savename`)))
  (if _returnvalue
    (bind _returnvalue_2 (`GameplayStatics.LoadGameFromSlot` (`self.savename`)))
    (bind _output_get (set `self.saveGameRef` _returnvalue_2))
    (bind _asbp_pinball_save (cast `/Game/MyContent/Blueprints/Pinball/BP_PinballSave` _output_get))
    (set `self.HighScore` (`/Game/MyContent/Blueprints/Pinball/BP_PinballSave.highScore` _asbp_pinball_save))))

(fn `Save`
  (bind _returnvalue (`GameplayStatics.DoesSaveGameExist` (`self.savename`)))
  (if _returnvalue
    (bind _returnvalue_2 (`GameplayStatics.LoadGameFromSlot` (`self.savename`)))
    (set `self.saveGameRef` _returnvalue_2)
    (else
      (bind _returnvalue_3 (`GameplayStatics.CreateSaveGameObject` "/Game/MyContent/Blueprints/Pinball/BP_PinballSave.BP_PinballSave_C"))
      (set `self.saveGameRef` _returnvalue_3)))
  (bind _asbp_pinball_save (cast `/Game/MyContent/Blueprints/Pinball/BP_PinballSave` (`self.saveGameRef`)))
  (set `/Game/MyContent/Blueprints/Pinball/BP_PinballSave.highScore` (`self.HighScore`) _asbp_pinball_save)
  (`GameplayStatics.SaveGameToSlot` (`self.saveGameRef`) (`self.savename`)))

(fn `UserConstructionScript`)