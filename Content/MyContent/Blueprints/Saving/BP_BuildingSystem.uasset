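; BP_BuildingSystem lets the player place a build in the world through a camera-aimed preview.
; While preview is toggled on, each Tick traces from the character's FollowCamera and moves or spawns the PreviewActor at the last hit location.
; ConfirmBuild spawns BuildClass there, ends preview and destroys the preview actor.
; Toggling preview off through ShowPreview only stops updates, leaving any preview actor in place.
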(event `self.ReceiveBeginPlay`
  (bind _asbp_third_person_character (cast `/Game/ThirdPerson/Blueprints/BP_ThirdPersonCharacter` (`GameplayStatics.GetPlayerCharacter` 0)))
  (set `self.BP_thirdPersonCharacter` _asbp_third_person_character))

(event `ShowPreview`
  (set `self.Preview` (not (`self.Preview`))))

(event `self.ReceiveTick`
  (params (DeltaSeconds :type "Float (single-precision)"))
  (if (`self.Preview`)
    (`self.PreviewLoop`)))

(event `PreviewLoop`
  (bind (_returnvalue_location _returnvalue_rotation) (`KismetMathLibrary.BreakTransform` (`SceneComponent.K2_GetComponentToWorld` (`/Game/ThirdPerson/Blueprints/BP_ThirdPersonCharacter.FollowCamera` (`self.BP_thirdPersonCharacter`)))))
  (bind (_outhit _returnvalue) (`KismetSystemLibrary.LineTraceSingle` _returnvalue_location (+ _returnvalue_location (* (`KismetMathLibrary.GetForwardVector` _returnvalue_rotation) 1000)) "TraceTypeQuery1" true (`|MakeArray` (`self.PreviewBuild`)) "ForDuration"))
  (if _returnvalue
    (set `self.Location` (`.Location` (`GameplayStatics.BreakHitResult` _outhit))))
  (if (`KismetSystemLibrary.IsValid` (`self.PreviewBuild`))
    (`Actor.K2_SetActorLocation` (`self.PreviewBuild`) (`self.Location`) false false)
    (else
      (bind _returnvalue_2 (`|SpawnActorFromClass` (`self.PreviewActor`) (`KismetMathLibrary.MakeTransform` (`self.Location`)) "Undefined" "MultiplyWithRoot" null null))
      (set `self.PreviewBuild` _returnvalue_2))))

(event `ConfirmBuild`
  (if (`self.Preview`)
    (`|SpawnActorFromClass` (`self.BuildClass`) (`KismetMathLibrary.MakeTransform` (`self.Location`)) "Undefined" "MultiplyWithRoot" null null)
    (set `self.Preview` false)
    (`Actor.K2_DestroyActor` (`self.PreviewBuild`))))