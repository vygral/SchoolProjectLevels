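; BP_startSequence is a trigger actor that plays an assigned level sequence when the player character enters its CollisionBox.
; On overlap, it disables the BP_ThirdPersonCharacter's input, plays PlayableSequence, waits for its duration via Delay, then re-enables input.
; The Once flag clears only after that delay, and input stays disabled if no valid sequence is set.
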(event `self.CollisionBox.OnComponentBeginOverlap`
  (params (OverlappedComponent :type "PrimitiveComponent Object Reference") (OtherActor :type "Actor Object Reference") (OtherComp :type "PrimitiveComponent Object Reference") (OtherBodyIndex :type Integer) (bFromSweep :type Boolean) (SweepResult :type "HitResult Structure (by ref)"))
  (bind _returnvalue (`GameplayStatics.GetPlayerCharacter` 0))
  (bind _playablesequence (`self.PlayableSequence`))
  (bind _sequenceplayer (`LevelSequenceActor.SequencePlayer` _playablesequence))
  (if (`self.once`)
    (if (== OtherActor _returnvalue)
      (bind _asbp_third_person_character (cast `/Game/ThirdPerson/Blueprints/BP_ThirdPersonCharacter` _returnvalue))
      (`self.DisableInput` _asbp_third_person_character null)
      (if (`KismetSystemLibrary.IsValid` _playablesequence)
        (`MovieSceneSequencePlayer.Play` _sequenceplayer)
        (`KismetSystemLibrary.Delay` (`TimeManagementBlueprintLibrary.Conv_QualifiedFrameTimeToSeconds` (`MovieSceneSequencePlayer.GetDuration` _sequenceplayer)))
        (`self.EnableInput` _asbp_third_person_character null)
        (set `self.once` false)))))

(fn `UserConstructionScript`)