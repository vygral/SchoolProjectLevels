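; BP_ScoreLevelOpener is a level exit pressure plate that loads a configured level once the player has enough points.
; When the player pawn overlaps it, it checks Points on the BP_Scoring game mode against PointsToOpen and opens LevelToOpen if met.
; Tick repeats that score check every frame to switch the plate to M_BaseMaterial once unlocked.
; The construction script fills two text renders with the display text and required points.
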(event `self.ReceiveBeginPlay`)

(event `self.ReceiveActorBeginOverlap`
  (params (OtherActor :type "Actor Object Reference"))
  (if (== OtherActor (`GameplayStatics.GetPlayerPawn` 0))
    (bind _asbp_scoring (cast `/Game/MyContent/Blueprints/BP_Scoring` (`GameplayStatics.GetGameMode`)))
    (if (>= (`/Game/MyContent/Blueprints/BP_Scoring.Points` _asbp_scoring) (`self.PointsToOpen`))
      (`GameplayStatics.OpenLevel` (`self.LevelToOpen`)))))

(event `self.ReceiveTick`
  (params (DeltaSeconds :type "Float (single-precision)"))
  (bind _asbp_scoring (cast `/Game/MyContent/Blueprints/BP_Scoring` (`GameplayStatics.GetGameMode`)))
  (if (>= (`/Game/MyContent/Blueprints/BP_Scoring.Points` _asbp_scoring) (`self.PointsToOpen`))
    (`PrimitiveComponent.SetMaterial` (`self.PressurePlate`) 0 "/Game/MyContent/Materials/M_BaseMaterial.M_BaseMaterial")))

(fn `UserConstructionScript`
  (`TextRenderComponent.K2_SetText` (`self.TextRender`) (`self.DisplayedText`))
  (`TextRenderComponent.K2_SetText` (`self.RequiredPoints`) (`KismetTextLibrary.Conv_StringToText` (`KismetStringLibrary.Concat_StrStr` (`KismetStringLibrary.Conv_IntToString` (`self.PointsToOpen`)) " Points"))))