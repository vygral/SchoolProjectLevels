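; BP_Explosion is an explosion actor that breaks Chaos destructibles and pushes physics objects when its Explode event is called.
; Explode spawns particles and sound at the Sphere, then applies an external cluster strain field with no falloff, sized by the Sphere's radius.
; It prints a debug string and waits one tick before firing the RadialForce impulse, so the push follows the strain field.
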(event `Explode`
  (bind _sphere (`self.Sphere`))
  (bind _returnvalue (`SceneComponent.K2_GetComponentLocation` _sphere))
  (`GameplayStatics.SpawnEmitterAtLocation` "/Game/StarterContent/Particles/P_Explosion.P_Explosion" _returnvalue)
  (`GameplayStatics.PlaySoundAtLocation` "/Game/StarterContent/Audio/Explosion01.Explosion01" _returnvalue (struct) 1.0 1.0 0.0 null null null null)
  (`FieldSystemComponent.ApplyPhysicsField` (`self.FieldSystemComponent`) true "Field_ExternalClusterStrain" null (`RadialFalloff.SetRadialFalloff` (`self.RadialFalloff`) 5000000.0 0.0 1.0 0.0 (`SphereComponent.GetScaledSphereRadius` _sphere) _returnvalue "Field_FallOff_None"))
  (`KismetSystemLibrary.PrintString` "Exposion")
  (`KismetSystemLibrary.DelayUntilNextTick`)
  (`RadialForceComponent.FireImpulse` (`self.RadialForce`)))

(fn `UserConstructionScript`)