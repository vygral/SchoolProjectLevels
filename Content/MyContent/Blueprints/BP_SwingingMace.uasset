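; BP_SwingingMace is a swinging hazard actor that restarts the current level when the player pawn overlaps it.
; Tick advances a speed-scaled timer, wrapped at two pi, and sets roll to its sine times MaxDegree while keeping pitch and yaw.
; The construction script applies SecondsOffset to the initial roll and adds it to the timer, setting the starting phase of the swing.
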(event `self.ReceiveBeginPlay`)

(event `self.ReceiveActorBeginOverlap`
  (params (OtherActor :type "Actor Object Reference"))
  (if (== OtherActor (`GameplayStatics.GetPlayerPawn` 0))
    (bind _returnvalue (`GameplayStatics.GetCurrentLevelName` true))
    (`GameplayStatics.OpenLevel` (`KismetStringLibrary.Conv_StringToName` _returnvalue))))

(event `self.ReceiveTick`
  (params (DeltaSeconds :type "Float (single-precision)"))
  (bind (_returnvalue_roll _returnvalue_pitch _returnvalue_yaw) (`KismetMathLibrary.BreakRotator` (`self.K2_GetActorRotation`)))
  (bind _seconds (`self.Seconds`))
  (bind _returnvalue (* (`KismetMathLibrary.GetPI`) 2.0))
  (bind _output_get (set `self.Seconds` (+ (* DeltaSeconds (`self.Speed`)) (`self.Seconds`))))
  (`self.K2_SetActorRotation` (`KismetMathLibrary.MakeRotator` (* (`KismetMathLibrary.Sin` _output_get) (`self.MaxDegree`)) _returnvalue_pitch _returnvalue_yaw))
  (if (>= _seconds _returnvalue)
    (set `self.Seconds` (- _seconds _returnvalue))))

(fn `UserConstructionScript`
  (`self.K2_SetActorRotation` (`KismetMathLibrary.MakeRotator` (* (`KismetMathLibrary.Sin` (`self.SecondsOffset`)) (`self.MaxDegree`))))
  (set `self.Seconds` (+ (`self.SecondsOffset`) (`self.Seconds`))))